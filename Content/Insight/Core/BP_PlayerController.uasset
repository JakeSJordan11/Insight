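; First-person-style player controller that handles movement, look, pausing and interaction.
; Enhanced Input drives yaw-relative movement and camera look, both gated by CrosshairVisible, which CreateCrosshair sets when it adds the crosshair widget.
; The pause action toggles game pause and a lazily created menu, opening only while that flag is set.
; Activate fills the crosshair and sends InteractMessage to the actor hit by a visibility line trace from the view point.
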(event `EnhancedInput|/Game/Insight/Core/Inputs/IA_WalkForward`
  (params (ActionValue :type "Float (double-precision)") (ElapsedSeconds :type "Float (double-precision)") (TriggeredSeconds :type "Float (double-precision)") (InputAction :type "InputAction Object Reference" :default "/Game/Insight/Core/Inputs/IA_WalkForward.IA_WalkForward"))
  ;[0.25 0.25 0.25 0.25] Movement
  (:`Triggered`
    (if (`self.bCrosshairVisible`)
      (`Pawn.AddMovementInput` (`self.K2_GetPawn`) (`KismetMathLibrary.GetForwardVector` (`KismetMathLibrary.MakeRotator` 0.0 0.0 (.yaw (`self.GetControlRotation`)))) ActionValue false))))

(event `EnhancedInput|/Game/Insight/Core/Inputs/IA_WalkRight`
  (params (ActionValue :type "Float (double-precision)") (ElapsedSeconds :type "Float (double-precision)") (TriggeredSeconds :type "Float (double-precision)") (InputAction :type "InputAction Object Reference" :default "/Game/Insight/Core/Inputs/IA_WalkRight.IA_WalkRight"))
  ;[0.25 0.25 0.25 0.25] Movement
  (:`Triggered`
    (if (`self.bCrosshairVisible`)
      (`Pawn.AddMovementInput` (`self.K2_GetPawn`) (`KismetMathLibrary.GetRightVector` (`KismetMathLibrary.MakeRotator` 0.0 0.0 (.yaw (`self.GetControlRotation`)))) ActionValue false))))

(event `EnhancedInput|/Game/Insight/Core/Inputs/IA_LookUp`
  (params (ActionValue :type "Float (double-precision)") (ElapsedSeconds :type "Float (double-precision)") (TriggeredSeconds :type "Float (double-precision)") (InputAction :type "InputAction Object Reference" :default "/Game/Insight/Core/Inputs/IA_LookUp.IA_LookUp"))
  ;[0.25 0.25 0.25 0.25] Look Around
  (:`Triggered`
    (if (`self.bCrosshairVisible`)
      (`self.AddPitchInput` ActionValue))))

(event `EnhancedInput|/Game/Insight/Core/Inputs/IA_LookRight`
  (params (ActionValue :type "Float (double-precision)") (ElapsedSeconds :type "Float (double-precision)") (TriggeredSeconds :type "Float (double-precision)") (InputAction :type "InputAction Object Reference" :default "/Game/Insight/Core/Inputs/IA_LookRight.IA_LookRight"))
  ;[0.25 0.25 0.25 0.25] Look Around
  (:`Triggered`
    (if (`self.bCrosshairVisible`)
      (`self.AddYawInput` ActionValue))))

(event `EnhancedInput|/Game/Insight/Core/Inputs/IA_Pause`
  (params (ActionValue :type Boolean) (ElapsedSeconds :type "Float (double-precision)") (TriggeredSeconds :type "Float (double-precision)") (InputAction :type "InputAction Object Reference" :default "/Game/Insight/Core/Inputs/IA_Pause.IA_Pause"))
  (bind _pausemenuref (`self.PauseMenuRef`))
  ;[0.25 0.25 0.25 0.25] Pause Menu
  (:`Started`
    (if (`self.bPaused`)
      (`GameplayStatics.SetGamePaused` false)
      (set `self.bPaused` false)
      (`Widget.RemoveFromParent` (`self.PauseMenuRef`))
      (elif (`self.bCrosshairVisible`)
        (`/Engine/EditorBlueprintResources/StandardMacros.IsValid` (`self.PauseMenuRef`)
          (:`Is Valid`
            _)
          (:`Is Not Valid`
            (bind _returnvalue (`|CreateWidget` "/Game/Insight/Core/WBP_PauseMenu.WBP_PauseMenu_C"))
            (set `self.PauseMenuRef` _returnvalue)))
        (set `self.bShowMouseCursor` true)
        (`WidgetBlueprintLibrary.SetInputMode_GameAndUIEx` (`GameplayStatics.GetPlayerController` 0) _pausemenuref)
        (`UserWidget.AddToViewport` _pausemenuref 0)
        (`GameplayStatics.SetGamePaused` true)
        (set `self.bPaused` true)))))

(event `CreateCrosshair`
  ;[0.251 0.251 0.251 0.25] Implement Crosshair
  (bind _returnvalue (`|CreateWidget` "/Game/Insight/Core/WBP_Crosshair.WBP_Crosshair_C"))
  (bind _output_get (set `self.CrosshairRef` _returnvalue))
  (`UserWidget.AddToViewport` _output_get 0)
  (set `self.bCrosshairVisible` true))

(event `EnhancedInput|/Game/Insight/Core/Inputs/IA_Activate`
  (params (ActionValue :type Boolean) (ElapsedSeconds :type "Float (double-precision)") (TriggeredSeconds :type "Float (double-precision)") (InputAction :type "InputAction Object Reference" :default "/Game/Insight/Core/Inputs/IA_Activate.IA_Activate"))
  (bind _crosshairref (`self.CrosshairRef`))
  (bind _crosshairref_2 (`self.CrosshairRef`))
  ;[0.251 0.251 0.251 0.25] Implement Crosshair
  (:`Started`
    (`/Engine/EditorBlueprintResources/StandardMacros.IsValid` _crosshairref
      (:`Is Valid`
        (`/Game/Insight/Core/WBP_Crosshair.FillCrossHairOn` _crosshairref)
        (bind _onhithitactor (`self.TraceForInteraction`)
          (:`Is Valid`
            (message `/Game/Insight/Core/BPI_Interactable.Interact` _onhithitactor))))))
  (:`Completed`
    (`/Engine/EditorBlueprintResources/StandardMacros.IsValid` _crosshairref_2
      (:`Is Valid`
        (`/Game/Insight/Core/WBP_Crosshair.FillCrosshairOff` _crosshairref_2)))))

(fn `UserConstructionScript`)